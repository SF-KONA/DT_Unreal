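; Robot arm Blueprint that reaches for a target actor, fakes picking it up and returns to idle.
; A timeline lerps EffectorLocation from a fixed rest point to the target's position relative to the arm, and reverses for idle.
; Each update pushes that location into the cached ABP_IndustrialRobot_IK instance, as does the construction script.
; Pickup hides the target and shows a stand-in cube matching its rotation.
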(event `RefreshAnimation`
  (bind _animblueprint (`self.GetAnimInstance`))
  (set `/Game/Blueprint/RobotArm/ABP_IndustrialRobot_IK.EffectorLocation` (`self.EffectorLocation`) _animblueprint))

(event `MoveToTargetActor`
  (`SceneComponent.K2_SetWorldLocation` (`self.TargetlocationInWorld`) (`self.K2_GetActorLocation` (`self.TargetActor`)) false false)
  (bind (_direction _newtrack_0) (`Timeline|MoveToTargetTimeline` :!label _label)
    (:`Update`
      (set `self.EffectorLocation` (`KismetMathLibrary.VLerp` (0.0 250.0 300.0) (`SceneComponent.RelativeLocation` (`self.TargetlocationInWorld`)) _newtrack_0))
      (`self.RefreshAnimation`))))

(event `ReturnToIdle`
  (goto _label :!via `Reverse`))

(event `Pickup`
  (`SceneComponent.K2_SetWorldRotation` (`self.Cube`) (`self.K2_GetActorRotation` (`self.TargetActor`)) false false)
  (`self.SetActorHiddenInGame` (`self.TargetActor`) true)
  (`SceneComponent.SetVisibility` (`self.Cube`) true false))

(fn `UserConstructionScript`
  (`self.RefreshAnimation`))